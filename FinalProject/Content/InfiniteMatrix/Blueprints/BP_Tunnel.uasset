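; BP_Tunnel is an endless-tunnel segment with a rotating holed wall, spinning health pack and enemy.
; Its end trigger asks TunnelSpawner for another segment, destroys itself, and rewards clean passes with score and capped speed gains.
; Overlaps damage or heal the player, absorb projectiles at walls, and award score for shot enemies.
; RandomizeWallHP picks the wall mesh and roll, and randomly places optional health pack and enemy.
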(event OnComponentBeginOverlap(TriggerZone)
  (params (OverlappedComponent :type Primitive%20Component%20Object%20Reference) (OtherActor :type Actor%20Object%20Reference) (OtherComp :type Primitive%20Component%20Object%20Reference) (OtherBodyIndex :type Integer) (bFromSweep :type Boolean) (SweepResult :type Hit%20Result%20Structure%20%28by%20ref%29))
  (bind _asbp_player (Utilities|Casting|CastToBP_Player OtherActor))
  ;[1 1 1] Core gameplay loop; respawn tunnels, increment speed, increment score if successful passthrough; reset wall monitor if hit wall
  (Default|SpawnTunnelatSpawnPoint (Variables|Default|GetTunnelSpawner))
  (Actor|DestroyActor)
  (if (Variables|Default|GetWallWasHit)
    (Variables|Default|SetWallWasHit false)
    (else
      (Default|IncrementScore _asbp_player)
      (if (<= (+ (Variables|/Game/InfiniteMatrix/Blueprints/BP_Player.BP_Player_C|GetPlayerSpeed _asbp_player) 5e+01) 5e+03)
        (Variables|/Game/InfiniteMatrix/Blueprints/BP_Player.BP_Player_C|SetPlayerSpeed _asbp_player (+ (Variables|/Game/InfiniteMatrix/Blueprints/BP_Player.BP_Player_C|GetPlayerSpeed _asbp_player) 5e+01))
        (else
          (Variables|/Game/InfiniteMatrix/Blueprints/BP_Player.BP_Player_C|SetPlayerSpeed _asbp_player 5e+03))))))

(event OnComponentBeginOverlap(HP_Mesh)
  (params (OverlappedComponent :type Primitive%20Component%20Object%20Reference) (OtherActor :type Actor%20Object%20Reference) (OtherComp :type Primitive%20Component%20Object%20Reference) (OtherBodyIndex :type Integer) (bFromSweep :type Boolean) (SweepResult :type Hit%20Result%20Structure%20%28by%20ref%29))
  (bind _asbp_player (Utilities|Casting|CastToBP_Player OtherActor))
  (Default|IncreaseHealth _asbp_player))

(event OnComponentBeginOverlap(EnemyMesh)
  (params (OverlappedComponent :type Primitive%20Component%20Object%20Reference) (OtherActor :type Actor%20Object%20Reference) (OtherComp :type Primitive%20Component%20Object%20Reference) (OtherBodyIndex :type Integer) (bFromSweep :type Boolean) (SweepResult :type Hit%20Result%20Structure%20%28by%20ref%29))
  (bind _asbp_player (Utilities|Casting|CastToBP_Player OtherActor)
    (:then
      (Default|DecreaseHealth _asbp_player))
    (:CastFailed
      (bind _asbp_projectile (Utilities|Casting|CastToBP_Projectile OtherActor))
      (bind _returnvalue (Actor|GetActorOfClass "/Game/InfiniteMatrix/Blueprints/BP_Player.BP_Player_C"))
      (Default|IncrementScore _returnvalue)))
  (Components|StaticMesh|SetStaticMesh (Variables|Default|GetEnemyMesh) 0)
  (Actor|DestroyActor _asbp_projectile))

(event OnComponentBeginOverlap(WallMesh)
  (params (OverlappedComponent :type Primitive%20Component%20Object%20Reference) (OtherActor :type Actor%20Object%20Reference) (OtherComp :type Primitive%20Component%20Object%20Reference) (OtherBodyIndex :type Integer) (bFromSweep :type Boolean) (SweepResult :type Hit%20Result%20Structure%20%28by%20ref%29))
  (bind _asbp_player (Utilities|Casting|CastToBP_Player OtherActor)
    (:then
      (Default|DecreaseHealth _asbp_player)
      (Variables|Default|SetWallWasHit true))
    (:CastFailed
      (bind _asbp_projectile (Utilities|Casting|CastToBP_Projectile OtherActor))
      (Actor|DestroyActor _asbp_projectile))))

(event EventTick
  (params (DeltaSeconds :type Float%20%28single-precision%29))
  ;[1 1 1] Wall and Medpack rotator
  (Utilities|FlowControl|Sequence
    (:then_0
      (Transformation|AddLocalRotation (Variables|Default|GetHP_Mesh) (Math|Rotator|MakeRotator 0.0 0.0 (* (Variables|Default|GetEntityRotateSpeed) DeltaSeconds)) false false))
    (:then_1
      (Transformation|AddLocalRotation (Variables|Default|GetWallMesh) (Math|Rotator|MakeRotator (* DeltaSeconds (Variables|Default|GetWallRotateSpeed)) 0.0 0.0) false false))))

(fn ConstructionScript)

(fn RandomizeWall&HP
  (bind _returnvalue (Math|Random|RandomFloatinRange -2e+02 2e+02))
  (bind _returnvalue_2 (Math|Random|RandomFloatinRange -3e+02 3e+02))
  (bind _hp_mesh (Variables|Default|GetHP_Mesh))
  (Utilities|FlowControl|Sequence
    (:then_0
      ;[1 1 1] Random Spawn Walls
      (Components|StaticMesh|SetStaticMesh (Variables|Default|GetWallMesh) (Utilities|Select :Index (Math|Random|RandomIntegerinRange 0 3) :Option%200 "/Game/InfiniteMatrix/Meshes/SM_Hole_01.SM_Hole_01" :Option%201 "/Game/InfiniteMatrix/Meshes/SM_Hole_02.SM_Hole_02" :Option%202 "/Game/InfiniteMatrix/Meshes/SM_Hole_03.SM_Hole_03" :Option%203 "/Game/InfiniteMatrix/Meshes/SM_Hole_04.SM_Hole_04"))
      (Transformation|AddLocalRotation (Variables|Default|GetWallMesh) (Math|Rotator|MakeRotator (Math|Random|RandomFloatinRange 0.0 3.6e+02) 0.0 0.0) false false))
    (:then_1
      ;[1 1 1] Random Spawn HP Location; set rotation speed
      (if (< (Math|Random|RandomIntegerinRange 0 10) 3)
        (Components|StaticMesh|SetStaticMesh _hp_mesh "/Game/InfiniteMatrix/Meshes/Healthpack.Healthpack")
        (Transformation|SetRelativeLocation _hp_mesh (Math|Vector|MakeVector (Math|Random|RandomFloatinRange 1e+03 2e+03) _returnvalue_2 _returnvalue_2) false false)
        (Transformation|AddLocalRotation _hp_mesh (Math|Rotator|MakeRotator 0.0 0.0 1.8e+02) false false)))
    (:then_2
      ;[1 1 1] Randomize Enemy Spawn
      (if (< (Math|Random|RandomIntegerinRange 0 10) 7)
        (Components|StaticMesh|SetStaticMesh (Variables|Default|GetEnemyMesh) "/Game/InfiniteMatrix/Meshes/Koffing.Koffing")
        (Transformation|SetRelativeLocation (Variables|Default|GetEnemyMesh) (Math|Vector|MakeVector (Math|Random|RandomFloatinRange 1e+03 2e+03) _returnvalue _returnvalue) false false)))))