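; Auto-scrolling camera actor that advances along +X and culls projectiles and enemies through overlap planes.
; Each Tick it eases toward a point 100 units ahead with FInterpTo, moving only while short of the level's BP_CamStop.
; PlaneB destroys bullets immediately and turrets, rotating turrets and moving enemies through one shared five-second Delay.
; PlaneT destroys any BP_Projectile that overlaps it.
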(event OnComponentBeginOverlap(PlaneB)
  (params (OverlappedComponent :type Primitive%20Component%20Object%20Reference) (OtherActor :type Actor%20Object%20Reference) (OtherComp :type Primitive%20Component%20Object%20Reference) (OtherBodyIndex :type Integer) (bFromSweep :type Boolean) (SweepResult :type Hit%20Result%20Structure%20%28by%20ref%29))
  ;[1 1 1] Enemy Culling
  (bind _asbp_bullet (Utilities|Casting|CastTobp_bullet OtherActor)
    (:then
      (Actor|DestroyActor _asbp_bullet))
    (:CastFailed
      (bind _asbp_turret (Utilities|Casting|CastTobp_turret OtherActor)
        (:then
          _)
        (:CastFailed
          (bind _asbp_rotaturret (Utilities|Casting|CastTobp_rotaturret OtherActor)
            (:then
              _)
            (:CastFailed
              (bind _asbp_movinenemy (Utilities|Casting|CastTobp_movinenemy OtherActor))))))
      (Utilities|FlowControl|Delay 5.0)
      (Actor|DestroyActor _asbp_turret))))

(event OnComponentBeginOverlap(PlaneT)
  (params (OverlappedComponent :type Primitive%20Component%20Object%20Reference) (OtherActor :type Actor%20Object%20Reference) (OtherComp :type Primitive%20Component%20Object%20Reference) (OtherBodyIndex :type Integer) (bFromSweep :type Boolean) (SweepResult :type Hit%20Result%20Structure%20%28by%20ref%29))
  (bind _asbp_projectile (Utilities|Casting|CastToBP_Projectile OtherActor))
  (Actor|DestroyActor _asbp_projectile))

(event EventBeginPlay)

(event Collision|EventActorBeginOverlap
  (params (OtherActor :type Actor%20Object%20Reference)))

(event EventTick
  (params (DeltaSeconds :type Float%20%28single-precision%29))
  (bind _returnvalue (Transformation|GetActorLocation))
  (bind _returnvalue_2 (+ (.x _returnvalue) 1e+02))
  (bind _returnvalue_3 (Math|Interpolation|FInterpTo (.x _returnvalue) _returnvalue_2 DeltaSeconds 2.0))
  ;[1 1 1] Camera Movement
  (bind _returnvalue_4 (Actor|GetActorOfClass "/Game/Blueprints/Triggers/BP_CamStop.BP_CamStop_C"))
  (if (< _returnvalue_3 (.x (Transformation|GetActorLocation _returnvalue_4)))
    (Transformation|SetActorLocation (Math|Vector|MakeVector _returnvalue_3 (.y _returnvalue) (.z _returnvalue)) false false)))

(fn ConstructionScript)