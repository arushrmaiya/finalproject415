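; Boss enemy that advances steadily along world X while firing bullets and tracking its health on a widget bar.
; A Delay on Tick throttles volleys from AutoFire's child arrows; nested inside that loop, AimFire's arrows turn toward the player and fire, once per AutoFire arrow.
; Projectile overlaps on its box reduce health and update the bar; at zero it destroys itself and calls ScoreUp on the player.
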(event OnComponentBeginOverlap(Box)
  (params (OverlappedComponent :type Primitive%20Component%20Object%20Reference) (OtherActor :type Actor%20Object%20Reference) (OtherComp :type Primitive%20Component%20Object%20Reference) (OtherBodyIndex :type Integer) (bFromSweep :type Boolean) (SweepResult :type Hit%20Result%20Structure%20%28by%20ref%29))
  (Utilities|Casting|CastToBP_Projectile OtherActor)
  (bind _output_get (Variables|Default|SetHealth (Math|Integer|Clamp(Integer) (- (Variables|Default|GetHealth) 2) 0 100)))
  (if (== _output_get 0)
    (Actor|DestroyActor)
    (bind _asbp_player_zd (Utilities|Casting|CastToBP_PlayerZD (Game|Player|GetPlayerPawn 0)))
    (Default|ScoreUp _asbp_player_zd)
    (else
      (bind _aswbp_enemy_health (Utilities|Casting|CastToWBP_EnemyHealth (UserInterface|GetWidget (Variables|Default|GetHealthBarWidget))))
      (Variables|/Script/UMG.ProgressBar|SetPercent (Variables|/Game/UI/Enemy/WBP_EnemyHealth.WBP_EnemyHealth_C|GetHealthBar _aswbp_enemy_health) (/ (Math|Conversions|ToFloat(Integer) (Variables|Default|GetHealth)) 1e+02)))))

(event EventBeginPlay
  (Variables|Default|SetHealth 100)
  (bind _aswbp_enemy_health (Utilities|Casting|CastToWBP_EnemyHealth (UserInterface|GetWidget (Variables|Default|GetHealthBarWidget))))
  (Variables|/Script/UMG.ProgressBar|SetPercent (Variables|/Game/UI/Enemy/WBP_EnemyHealth.WBP_EnemyHealth_C|GetHealthBar _aswbp_enemy_health) 1.0))

(event EventTick
  (params (DeltaSeconds :type Float%20%28single-precision%29))
  (bind _returnvalue (Transformation|GetActorLocation))
  (Transformation|SetActorLocation (Math|Vector|MakeVector (Math|Interpolation|FInterpTo (.x _returnvalue) (+ (.x _returnvalue) 1e+02) DeltaSeconds 2.0) (.y _returnvalue) (.z _returnvalue)) false false)
  (Utilities|FlowControl|Delay 0.3)
  (for _array_element (Components|GetChildrenComponents (Variables|Default|GetAutoFire) false)
    (bind _asarrow_component (Utilities|Casting|CastToArrowComponent _array_element))
    (CallFunction|FireWeapon _asarrow_component)
    (for _array_element_2 (Components|GetChildrenComponents (Variables|Default|GetAimFire) false)
      (bind _asarrow_component_2 (Utilities|Casting|CastToArrowComponent _array_element_2))
      (CallFunction|AimWeapon _asarrow_component_2))))

(fn ConstructionScript)

(fn FireWeapon
  (params (ArrowIn :type Arrow%20Component%20Object%20Reference))
  (Game|SpawnActorfromClass "/Game/Blueprints/Enemies/bp_bullet.bp_bullet_C" (Transformation|GetWorldTransform ArrowIn) "Undefined" "MultiplyWithRoot" 0 0))

(fn AimWeapon
  (params (ArrowIn :type Arrow%20Component%20Object%20Reference))
  (bind _returnvalue (Game|Player|GetPlayerPawn 0))
  (Utilities|Casting|CastToBP_PlayerZD _returnvalue)
  (Transformation|SetWorldRotation ArrowIn (Math|Rotator|FindLookatRotation (Transformation|GetWorldLocation ArrowIn) (Transformation|GetActorLocation _returnvalue)) false false)
  (Game|SpawnActorfromClass "/Game/Blueprints/Enemies/bp_bullet.bp_bullet_C" (Transformation|GetWorldTransform ArrowIn) "Undefined" "MultiplyWithRoot" 0 0))