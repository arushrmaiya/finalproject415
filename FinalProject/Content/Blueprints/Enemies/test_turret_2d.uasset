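; Enemy turret that faces the player, fires bullets and awards score when killed.
; Tick turns the actor toward BP_PlayerZD, with a Delay throttling Bp_bullet spawns from the Arrow component.
; BP_Projectile overlaps on the Box reduce health and update the WBP_EnemyHealth bar.
; At zero health it sets IsDead, then after a short delay destroys itself and calls ScoreUp on the player.
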(event OnComponentBeginOverlap(Box)
  (params (OverlappedComponent :type Primitive%20Component%20Object%20Reference) (OtherActor :type Actor%20Object%20Reference) (OtherComp :type Primitive%20Component%20Object%20Reference) (OtherBodyIndex :type Integer) (bFromSweep :type Boolean) (SweepResult :type Hit%20Result%20Structure%20%28by%20ref%29))
  (Utilities|Casting|CastToBP_Projectile OtherActor)
  (bind _output_get (Variables|Default|SetHealth (Math|Integer|Clamp(Integer) (- (Variables|Default|GetHealth) 10) 0 100)))
  (if (== _output_get 0)
    (Variables|Default|SetIsDead true)
    (Utilities|FlowControl|Delay 0.2)
    (Actor|DestroyActor)
    (bind _asbp_player_zd (Utilities|Casting|CastToBP_PlayerZD (Game|Player|GetPlayerPawn 0)))
    (Default|ScoreUp _asbp_player_zd)
    (else
      (bind _aswbp_enemy_health (Utilities|Casting|CastToWBP_EnemyHealth (UserInterface|GetWidget (Variables|Default|GetHealthBarWidget))))
      (Variables|/Script/UMG.ProgressBar|SetPercent (Variables|/Game/UI/Enemy/WBP_EnemyHealth.WBP_EnemyHealth_C|GetHealthBar _aswbp_enemy_health) (/ (Math|Conversions|ToFloat(Integer) (Variables|Default|GetHealth)) 1e+02)))))

(event EventBeginPlay
  (Variables|Default|SetHealth 100)
  (bind _aswbp_enemy_health (Utilities|Casting|CastToWBP_EnemyHealth (UserInterface|GetWidget (Variables|Default|GetHealthBarWidget))))
  (Variables|/Script/UMG.ProgressBar|SetPercent (Variables|/Game/UI/Enemy/WBP_EnemyHealth.WBP_EnemyHealth_C|GetHealthBar _aswbp_enemy_health) 1.0)
  (Variables|Default|SetShootAnim false)
  (Variables|Default|SetIsDead false))

(event Collision|EventActorBeginOverlap
  (params (OtherActor :type Actor%20Object%20Reference)))

(event EventTick
  (params (DeltaSeconds :type Float%20%28single-precision%29))
  (bind _returnvalue (Game|Player|GetPlayerPawn 0))
  (Utilities|Casting|CastToBP_PlayerZD _returnvalue)
  (Transformation|SetActorRotation (Math|Rotator|FindLookatRotation (Transformation|GetActorLocation) (Transformation|GetActorLocation _returnvalue)))
  (Utilities|FlowControl|Delay 0.5)
  (Variables|Default|SetShootAnim true)
  (Game|SpawnActorfromClass "/Game/Blueprints/Enemies/bp_bullet.bp_bullet_C" (Transformation|GetWorldTransform (Variables|Default|GetArrow)) "Undefined" "MultiplyWithRoot" 0 0))

(fn ConstructionScript)