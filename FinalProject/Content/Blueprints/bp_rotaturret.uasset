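; Turret actor that fires continuously and can be destroyed by projectiles.
; Tick runs through a short Delay, which throttles spawning of Bp_bullet at the Arrow component's transform to about ten shots per second.
; BP_Projectile overlaps on the Box component reduce a clamped Health value, and the turret destroys itself when it reaches zero.
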(event OnComponentBeginOverlap(Box)
  (params (OverlappedComponent :type Primitive%20Component%20Object%20Reference) (OtherActor :type Actor%20Object%20Reference) (OtherComp :type Primitive%20Component%20Object%20Reference) (OtherBodyIndex :type Integer) (bFromSweep :type Boolean) (SweepResult :type Hit%20Result%20Structure%20%28by%20ref%29))
  (Utilities|Casting|CastToBP_Projectile OtherActor)
  (bind _output_get (Variables|Default|SetHealth (Math|Integer|Clamp(Integer) (- (Variables|Default|GetHealth) 10) 0 100)))
  (if (== _output_get 0)
    (Actor|DestroyActor)
    (Actor|DestroyActor)))

(event EventBeginPlay
  (Variables|Default|SetHealth 100))

(event Collision|EventActorBeginOverlap
  (params (OtherActor :type Actor%20Object%20Reference)))

(event EventTick
  (params (DeltaSeconds :type Float%20%28single-precision%29))
  (Utilities|FlowControl|Delay 0.1)
  (Game|SpawnActorfromClass "/Game/Blueprints/bp_bullet.bp_bullet_C" (Transformation|GetWorldTransform (Variables|Default|GetArrow)) "Undefined" "MultiplyWithRoot" 0 0))

(fn ConstructionScript)